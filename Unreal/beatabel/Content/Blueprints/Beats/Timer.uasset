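; Rhythm game beat timer: runs a countdown, plays the chosen song and scores Beat presses until the track ends.
; BeginPlay reads timestamps from MyGameInstance, and chained timers use each as the interval to the next beat.
; A rate-scaled timeline animates two boomboxes per beat; boombox scale at press time sets accuracy, score and GameMode message, one hit per beat.
; The HTTP timestamp request is disconnected.
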(event `ProcessGET`
  (params (Request :type "VaRestRequestJSON Object Reference"))
  ;[1 1 1] GET request for timestamps
  (bind _returnvalue (`VaRestRequestJSON.GetResponseObject` Request))
  (bind _output_get (set `self.responseObject` _returnvalue))
  (`|ExecutionSequence`
    (:`then_0`
      (for (_array_element _array_index) (`KismetStringLibrary.ParseIntoArray` (`KismetStringLibrary.Replace` (`KismetStringLibrary.Replace` (`VaRestJsonValue.AsString` (`VaRestJsonObject.GetField` (`|GetArrayItem` (`VaRestJsonObject.GetObjectArrayField` _output_get "Songs") 2) "timestamps")) "[") "]"))
        (`KismetArrayLibrary.Array_Insert` (`self.timestamps`) (`KismetStringLibrary.Conv_StringToDouble` _array_element) _array_index))
      (`KismetArrayLibrary.Array_Append` (`self.masterTimestamps`) (`self.timestamps`))
      (`KismetArrayLibrary.Array_Clear` (`self.timestamps`)))))

(event `CountDown`
  ;[1 1 1] Countdown
  (`/Game/Blueprints/GameMode.SetMessage` (stale `self.ReceiveBeginPlay` _asgame_mode) (`KismetStringLibrary.Conv_IntToString` (`self.CountdownValue`)))
  (`KismetSystemLibrary.K2_SetTimerDelegate` (delegate `DecrementCountDownValue`) 1.0 :!label _label))

(event `DecrementCountDownValue`
  (bind _countdownvalue (`self.CountdownValue`))
  ;[1 1 1] Countdown
  (bind _result (`/Engine/EditorBlueprintResources/StandardMacros.DecrementInt` _countdownvalue)
    (:`  `
      (set `self.CountdownValue` _result)
      (`/Game/Blueprints/GameMode.SetMessage` (stale `self.ReceiveBeginPlay` _asgame_mode) (`KismetStringLibrary.Conv_IntToString` _countdownvalue))
      (if (!= (`self.CountdownValue`) 0)
        (goto _label)
        (else
          (bind _asgame_mode (cast `/Game/Blueprints/GameMode` (`GameplayStatics.GetGameMode`)))
          (`/Game/Blueprints/GameMode.SetMessage` _asgame_mode "GO!!")
          (`self.EnableInput` (`GameplayStatics.GetPlayerCharacter` 0) (`GameplayStatics.GetPlayerController` 0))
          (bind _ascharacter (cast `/Game/Blueprints/Character/Character` (`GameplayStatics.GetPlayerPawn` 0)))
          (set `/Game/Blueprints/Character/Character.isPlaying` true _ascharacter)
          (`KismetSystemLibrary.K2_SetTimerDelegate` (delegate `StartSong`) 2.0))))))

(event `self.ReceiveBeginPlay`
  ;[1 1 1] Get timestamps of selected song from gameinstance
  (bind _asmy_game_instance (cast `/Game/Blueprints/DataStorage/MyGameInstance` (`GameplayStatics.GetGameInstance`)))
  (set `self.masterTimestamps` (`/Game/Blueprints/DataStorage/MyGameInstance.Timestamps` _asmy_game_instance))
  ;[1 1 1] Countdown
  (bind _asgame_mode (cast `/Game/Blueprints/GameMode` (`GameplayStatics.GetGameMode`)))
  (`/Game/Blueprints/GameMode.SetMessage` _asgame_mode "Get Ready!")
  (`KismetSystemLibrary.K2_SetTimerDelegate` (delegate `CountDown`) 2.0))

(event `InputAction|Beat`
  (params (Key :type "Key Structure"))
  ;[1 1 1] Score
  (:`Pressed`
    (if (`self.isHittable`)
      (bind _ascharacter (cast `/Game/Blueprints/Character/Character` (`GameplayStatics.GetPlayerPawn` 0)))
      (if (`/Game/Blueprints/Character/Character.isPlaying` _ascharacter)
        (set `self.isHittable` false) ; disables tap to avoid hitting more than once per beat
        (bind _asgame_mode (cast `/Game/Blueprints/GameMode` (`GameplayStatics.GetGameMode`)))
        (bind _output_get (set `self.accuracy` (`KismetMathLibrary.Abs` (- (.x (`SceneComponent.K2_GetComponentScale` (`self.Right boombox`))) 4.0))))
        (if (>= _output_get 3.0)
          (set `self.multiplier` 100.0)
          (`/Game/Blueprints/GameMode.SetMessage` _asgame_mode "GREAT!")
          (elif (>= _output_get 2.0)
            (set `self.multiplier` 10.0)
            (`/Game/Blueprints/GameMode.SetMessage` _asgame_mode "Good!")
            (else
              (`/Game/Blueprints/GameMode.SetMessage` _asgame_mode "Meh..."))))
        (`/Game/Blueprints/GameMode.AddScore` _asgame_mode (`KismetMathLibrary.FTrunc` (* (`self.multiplier`) (`self.accuracy`))))
        (set `self.multiplier` 0.0)))))

(event `StartSong`
  (bind _right_boombox (`self.Right boombox`))
  (bind _right_boombox_2 (`self.Right boombox`))
  (bind _output (`|GetArrayItem` (`self.masterTimestamps`) (`self.index`)))
  ;[1 1 1] Timer logic
  (bind _gameinstance (`self.GameInstanceGetter`))
  (`GameplayStatics.PlaySound2D` (`/Game/Blueprints/DataStorage/MyGameInstance.ChosenSongWav` _gameinstance) 1.0 1.0 0.0 null null)
  (set `self.TimeRemaining` (`KismetArrayLibrary.Array_Length` (`self.masterTimestamps`)))
  (bind _returnvalue (`KismetSystemLibrary.K2_SetTimerDelegate` (delegate `SetNextTimer`) _output :!label _label_2))
  ;[1 1 1] Animate boombox
  (`TimelineComponent.SetPlayRate` (`self.Resizing`) (/ 1.0 _output))
  (set `self.isHittable` true) ; enables tap
  (bind (_direction _emission _shrink _color) (`Timeline|Resizing` :!via `PlayFromStart`)
    (:`Update`
      (`SceneComponent.SetWorldScale3D` _right_boombox _shrink)
      (`SceneComponent.SetWorldScale3D` (`self.Left boombox`) _shrink)
      (`MeshComponent.SetVectorParameterValueOnMaterials` _right_boombox "Color" _color)
      (`MeshComponent.SetVectorParameterValueOnMaterials` (`self.Left boombox`) "Color" _color)
      (`MeshComponent.SetScalarParameterValueOnMaterials` _right_boombox "Emission" _emission)
      (`MeshComponent.SetScalarParameterValueOnMaterials` (`self.Left boombox`) "Emission" _emission))
    (:`Finished`
      (if (< (`KismetArrayLibrary.Array_Length` (`self.masterTimestamps`)) (`self.index`))
        (`SceneComponent.SetWorldScale3D` _right_boombox_2 (`self.Original Size`))
        (`SceneComponent.SetWorldScale3D` (`self.Left boombox`) (`self.Original Size`))
        (`MeshComponent.SetVectorParameterValueOnMaterials` _right_boombox_2 "Color" (0.0 1.0 0.0))
        (`MeshComponent.SetVectorParameterValueOnMaterials` (`self.Left boombox`) "Color" (0.0 1.0 0.0))))))

(event `SetNextTimer`
  ;[1 1 1] Timer logic
  (bind _result (`/Engine/EditorBlueprintResources/StandardMacros.IncrementInt` (`self.index`))
    (:`  `
      (bind _output_get (set `self.index` _result))
      (if (< _output_get (`KismetArrayLibrary.Array_Length` (`self.masterTimestamps`)))
        (`self.Decrement`)
        (goto _label_2)
        (else
          (`self.Decrement`)
          (`KismetSystemLibrary.K2_ClearAndInvalidateTimerHandle` (stale `StartSong` _returnvalue))
          (`KismetSystemLibrary.K2_SetTimerDelegate` (delegate `EndGame`) 2.0))))))

(event `EndGame`
  ;[1 1 1] End Game
  (`KismetSystemLibrary.PrintString` "Finished! ")
  (bind _ascharacter (cast `/Game/Blueprints/Character/Character` (`GameplayStatics.GetPlayerPawn` 0)))
  (set `/Game/Blueprints/Character/Character.isPlaying` false _ascharacter)
  (bind _asgame_mode (cast `/Game/Blueprints/GameMode` (`GameplayStatics.GetGameMode`)))
  (`/Game/Blueprints/GameMode.SetMessage` _asgame_mode "Thank you!!"))

(fn `Decrement`
  (bind _result (`/Engine/EditorBlueprintResources/StandardMacros.DecrementInt` (`self.TimeRemaining`))
    (:`  `
      (bind _output_get (set `self.TimeRemaining` _result))
      (`KismetSystemLibrary.PrintString` (`KismetStringLibrary.Concat_StrStr` "Timer at: " (`KismetStringLibrary.Conv_IntToString` _output_get))))))

(fn `GameInstanceGetter`
  (returns (GameInstance :type "/Game/Blueprints/DataStorage/MyGameInstance Object Reference"))
  (bind _asmy_game_instance (cast `/Game/Blueprints/DataStorage/MyGameInstance` (`GameplayStatics.GetGameInstance`)))
  (return _asmy_game_instance))

(fn `UserConstructionScript`)