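; REST test Blueprint that fetches song timestamp data from a web URL when the 2 key is pressed.
; It sends a VaRest-style GET request with custom headers and handles the JSON response in ProcessGET.
; Each entry in "Songs" has its timestamps string stripped of brackets, split and converted to floats, then appended to one MasterTimestamps array.
; A loop that prints those values is present but unconnected.
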(event `Key|Two`
  (params (Key :type "Key Structure"))
  (:`Pressed`
    (bind _output_get (set `self.Request` (`VaRestRequestJSON.ConstructRequestExt` "GET" "x_www_form_urlencoded_url")))
    (`VaRestRequestJSON.SetHeader` _output_get "Content-Type" "multipart/form-data")
    (`VaRestRequestJSON.SetHeader` _output_get "getDelta" "0")
    (add `VaRestRequestJSON.OnRequestComplete` _output_get (delegate `ProcessGET`))
    (`VaRestRequestJSON.ProcessURL` _output_get (`self.URL`))))

(event `ProcessGET`
  (params (Request :type "VaRestRequestJSON Object Reference"))
  (bind _returnvalue (`VaRestRequestJSON.GetResponseObject` Request))
  (bind _output_get (set `self.responseObject` _returnvalue))
  (for _array_element (`VaRestJsonObject.GetObjectArrayField` _output_get "Songs")
    (for (_array_element_2 _array_index) (`KismetStringLibrary.ParseIntoArray` (`KismetStringLibrary.Replace` (`KismetStringLibrary.Replace` (`VaRestJsonValue.AsString` (`VaRestJsonObject.GetField` _array_element "timestamps")) "[") "]"))
      (`KismetArrayLibrary.Array_Insert` (`self.timestamps`) (`KismetStringLibrary.Conv_StringToDouble` _array_element_2) _array_index))
    (`KismetArrayLibrary.Array_Append` (`self.masterTimestamps`) (`self.timestamps`))
    (`KismetArrayLibrary.Array_Clear` (`self.timestamps`))))

(fn `UserConstructionScript`)