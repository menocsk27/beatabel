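; Painting canvas actor that shows a random image on its Canvas mesh and the painted render target on its Plane through dynamic materials.
; DrawBrush, with no caller in this Blueprint, stamps a brush material onto the render target at a normalized location.
; NextImage exports the painting as a PNG named after the image with an unused number suffix, then rebuilds everything for another random image.
; Key 1 exports to a fixed filename.
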(event `self.ReceiveBeginPlay`
  (`|ExecutionSequence`
    (:`then_0`
      (bind _returnvalue (`KismetRenderingLibrary.CreateRenderTarget2D` 1024 1024 "RTF_RGBA8" :!label _label))
      (bind _output_get (set `self.RenderTarget` _returnvalue))
      (`KismetRenderingLibrary.ClearRenderTarget2D` _output_get))
    (:`then_1`
      (bind _returnvalue_2 (`KismetMaterialLibrary.CreateDynamicMaterialInstance` "/Game/Beatabel/Materials/Brush/M_Canvas.M_Canvas" :!label _label_2))
      (bind _randomtexture (`self.GetRandomTexture`))
      (set `self.ChosenFileName` (`KismetSystemLibrary.GetDisplayName` _randomtexture))
      (`MaterialInstanceDynamic.SetTextureParameterValue` _returnvalue_2 "RenderTarget" _randomtexture)
      (`PrimitiveComponent.SetMaterial` (`self.Canvas`) 0 _returnvalue_2))
    (:`then_2`
      (bind _returnvalue_3 (`KismetMaterialLibrary.CreateDynamicMaterialInstance` "/Game/Beatabel/Materials/Brush/M_Canvas_2.M_Canvas_2" :!label _label_3))
      (`MaterialInstanceDynamic.SetTextureParameterValue` _returnvalue_3 "RenderTarget" (`self.RenderTarget`))
      (`PrimitiveComponent.SetMaterial` (`self.Plane`) 0 _returnvalue_3))
    (:`then_3`
      (bind _returnvalue_4 (`KismetMaterialLibrary.CreateDynamicMaterialInstance` "/Game/Beatabel/Materials/Brush/M_Brush.M_Brush" :!label _label_4))
      (set `self.BrushMaterial` _returnvalue_4))))

(event `InputAction|NextImage`
  (params (Key :type "Key Structure"))
  (bind _returnvalue (`KismetStringLibrary.Concat_StrStr` (`self.Path`) "\\" (`KismetStringLibrary.Concat_StrStr` (`self.ChosenFileName`) "_" (`KismetStringLibrary.Conv_IntToString` (`self.fileNumber`))) ".png"))
  (:`Pressed`
    (`|ExecutionSequence`
      (:`then_0`
        (while (`BlueprintPathsLibrary.FileExists` _returnvalue)
          (bind _result (`/Engine/EditorBlueprintResources/StandardMacros.IncrementInt` (`self.fileNumber`))
            (:`  `
              (set `self.fileNumber` _result))))
        (bind _output_get (set `self.FileName` (`KismetStringLibrary.Concat_StrStr` (`BlueprintPathsLibrary.GetBaseFilename` _returnvalue) ".png")))
        (set `self.fileNumber` 0))
      (:`then_1`
        (`KismetRenderingLibrary.ExportRenderTarget` (`self.RenderTarget`) (`self.Path`) _output_get))
      (:`then_2`
        (goto _label))
      (:`then_3`
        (goto _label_2))
      (:`then_4`
        (goto _label_3))
      (:`then_5`
        (goto _label_4)))))

(event `Key|One`
  (params (Key :type "Key Structure"))
  ;[1 1 1] Save Texture
  (:`Pressed`
    (`KismetRenderingLibrary.ExportRenderTarget` (`self.RenderTarget`) (`self.Path`) "Texture.png")
    (`KismetSystemLibrary.PrintString` "Texture Saved")))

(fn `DrawBrush`
  (params (`Brush Texture` :type "Texture2D Object Reference") (`Brush Size` :type "Float (double-precision)") (`Draw Location` :type "Vector2D Structure"))
  (bind _brush_size (`local.Brush Size`))
  (`|ExecutionSequence`
    (:`then_0`
      (`MaterialInstanceDynamic.SetTextureParameterValue` (`self.BrushMaterial`) "BrushTexture" (`local.Brush Texture`)))
    (:`then_1`
      (bind (_canvas _size _context) (`KismetRenderingLibrary.BeginDrawCanvasToRenderTarget` (`self.RenderTarget`)))
      (`Canvas.K2_DrawMaterial` _canvas (`self.BrushMaterial`) (- (* _size (`local.Draw Location`)) (/ _brush_size 2.0)) (`KismetMathLibrary.MakeVector2D` _brush_size _brush_size) (0.0 0.0) (1.0 1.0) 0.0 (0.5 0.5))
      (`KismetRenderingLibrary.EndDrawCanvasToRenderTarget` _context))))

(fn `GetRandomTexture`
  (returns (RandomTexture :type "Texture2D Object Reference"))
  (return (`|GetArrayItem` (`self.RandomTextureArray`) (`KismetMathLibrary.RandomInteger` (`self.MapCount`)))))

(fn `UserConstructionScript`)